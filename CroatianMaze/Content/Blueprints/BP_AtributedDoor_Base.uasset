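; Base door actor with size, shape and colour attributes, each paired with a target value.
; On BeginPlay it derives a starting state from the targets through fixed mappings, so every attribute begins different from its target.
; ChangeAttributes stores the new values, then uses nested selects to set the wall mesh from size and shape and the door material from colour.
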(event `self.ReceiveBeginPlay`
  (`self.ChangeAttributes` (select `/Game/Blueprints/E_Size` (`self.TargetSize`) :`NewEnumerator0` "NewEnumerator1" :`NewEnumerator1` "NewEnumerator0" :!type "/Game/Blueprints/E_Size Enum") (select `/Game/Blueprints/E_Shape` (`self.TargetShape`) :`NewEnumerator0` "NewEnumerator2" :`NewEnumerator1` "NewEnumerator0" :`NewEnumerator2` "NewEnumerator1" :!type "/Game/Blueprints/E_Shape Enum") (select `/Game/Blueprints/E_Colour` (`self.TargetColour`) :`NewEnumerator0` "NewEnumerator3" :`NewEnumerator1` "NewEnumerator0" :`NewEnumerator3` "NewEnumerator1" :!type "/Game/Blueprints/E_Colour Enum")))

(fn `ChangeAttributes`
  (params (NewSize :type "/Game/Blueprints/E_Size Enum" :default "NewEnumerator0") (NewShape :type "/Game/Blueprints/E_Shape Enum" :default "NewEnumerator0") (NewColour :type "/Game/Blueprints/E_Colour Enum" :default "NewEnumerator0"))
  (bind _currentsize (`self.CurrentSize`))
  (bind _currentshape (`self.CurrentShape`))
  (bind _currentcolour (`self.CurrentColour`))
  (bind _output_get (set `self.CurrentSize` (select `bool` (`|EnumEquality` NewSize _currentsize) :`false` NewSize :`true` _currentsize)))
  (bind _output_get_2 (set `self.CurrentShape` (select `bool` (`|EnumEquality` NewShape _currentshape) :`false` NewShape :`true` _currentshape)))
  (set `self.CurrentColour` (select `bool` (`|EnumEquality` NewColour _currentcolour) :`false` NewColour :`true` _currentcolour))
  (`StaticMeshComponent.SetStaticMesh` (`self.WallMesh`) (select `/Game/Blueprints/E_Size` _output_get :`NewEnumerator0` (select `/Game/Blueprints/E_Shape` _output_get_2 :`NewEnumerator0` "/Game/Blueprints/DoorMeshes/SM_DoorSquareSmall.SM_DoorSquareSmall" :`NewEnumerator1` "/Game/Blueprints/DoorMeshes/SM_DoorCircleSmall.SM_DoorCircleSmall" :`NewEnumerator2` "/Game/Blueprints/DoorMeshes/SM_DoorTriangleSmall1.SM_DoorTriangleSmall1" :!type "StaticMesh Object Reference") :`NewEnumerator1` (select `/Game/Blueprints/E_Shape` _output_get_2 :`NewEnumerator0` "/Game/Blueprints/DoorMeshes/SM_DoorSquareBig.SM_DoorSquareBig" :`NewEnumerator1` "/Game/Blueprints/DoorMeshes/SM_DoorCircleBig.SM_DoorCircleBig" :`NewEnumerator2` "/Game/Blueprints/DoorMeshes/SM_DoorTriangleBig.SM_DoorTriangleBig" :!type "StaticMesh Object Reference")))
  (`PrimitiveComponent.SetMaterial` (`self.DoorMesh`) 0 (select `/Game/Blueprints/E_Colour` (`self.CurrentColour`) :`NewEnumerator0` "/Engine/MapTemplates/Materials/BasicAsset01.BasicAsset01" :`NewEnumerator1` "/Engine/MapTemplates/Materials/BasicAsset03.BasicAsset03" :`NewEnumerator3` "/Game/Blueprints/DoorMeshes/BasicAsset04.BasicAsset04" :!type "MaterialInterface Object Reference")))

(fn `UserConstructionScript`)